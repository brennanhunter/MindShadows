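; BP_Platform is an interactable platform that toggles between raised and lowered positions, starting from either one according to StartsUp.
; Interact alternates timelines forward and reverse to move the mesh in Z, swapping blue and white materials, with IsMoving blocking retriggers until shortly after completion.
; Timeline updates also call Interact on other platforms sharing its GroupTag, moving groups together.
; Shadow variants stay red and destroy the first-person character on hit.
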(event `/Game/Blueprints/Interfaces/BPI_Interact.Interact`
  (if (not (`self.isMoving`))
    (set `self.isMoving` true)
    (if (not (`self.StartsUp?`))
      (if (not (`self.isShadow`))
        (`/Engine/EditorBlueprintResources/StandardMacros.FlipFlop`
          (:`A`
            (`PrimitiveComponent.SetMaterial` (`self.Platform`) 0 "/Game/Materials/Platforms/M_Blue.M_Blue")
            (bind (_direction _timetogrow) (`Timeline|StartDownTimeline` :!label _label)
              (:`Update`
                (`SceneComponent.K2_SetRelativeLocation` (`self.Platform`) (`KismetMathLibrary.MakeVector` 0.0 0.0 (* _timetogrow (`self.AmountToGrow`))) false false)
                (bind _outactors (`GameplayStatics.GetAllActorsOfClass` "BP_Platform_C" :!label _label_2))
                (`self.InteractWithGroup` _outactors))
              (:`Finished`
                (`KismetSystemLibrary.Delay` 0.2 :!label _label_3)
                (set `self.isMoving` false))))
          (:`B`
            (`PrimitiveComponent.SetMaterial` (`self.Platform`) 0 "/Game/Materials/Platforms/M_DefaultWhite.M_DefaultWhite")
            (goto _label :!via `Reverse`)))
        (else
          (`/Engine/EditorBlueprintResources/StandardMacros.FlipFlop`
            (:`A`
              (goto _label))
            (:`B`
              (goto _label :!via `Reverse`)))))
      (elif (not (`self.isShadow`))
        (`/Engine/EditorBlueprintResources/StandardMacros.FlipFlop`
          (:`A`
            (`PrimitiveComponent.SetMaterial` (`self.Platform`) 0 "/Game/Materials/Platforms/M_DefaultWhite.M_DefaultWhite")
            (bind (_direction_2 _timetogrow_2) (`Timeline|StartUpTimeline` :!label _label_4)
              (:`Update`
                (`SceneComponent.K2_SetRelativeLocation` (`self.Platform`) (`KismetMathLibrary.MakeVector` 0.0 0.0 (* _timetogrow_2 (`self.AmountToShrink`))) false false)
                (goto _label_2))
              (:`Finished`
                (goto _label_3))))
          (:`B`
            (`PrimitiveComponent.SetMaterial` (`self.Platform`) 0 "/Game/Materials/Platforms/M_Blue.M_Blue")
            (goto _label_4 :!via `Reverse`)))
        (else
          (`/Engine/EditorBlueprintResources/StandardMacros.FlipFlop`
            (:`A`
              (goto _label_4))
            (:`B`
              (goto _label_4 :!via `Reverse`))))))))

(event `self.Platform.OnComponentHit`
  (params (HitComponent :type "PrimitiveComponent Object Reference") (OtherActor :type "Actor Object Reference") (OtherComp :type "PrimitiveComponent Object Reference") (NormalImpulse :type "Vector Structure") (Hit :type "HitResult Structure (by ref)"))
  (if (`self.isShadow`)
    (`self.K2_DestroyActor` (cast `/Game/FirstPerson/Blueprints/BP_FirstPersonCharacter` OtherActor :!pure true))))

(fn `InteractWithGroup`
  (params (Array :type "Array of /Game/Blueprints/Platforms/BP_Platform Object Reference"))
  (for _array_element Array
    (if (and (!= self _array_element) (`KismetStringLibrary.EqualEqual_StrStr` (`self.GroupTag`) (`/Game/Blueprints/Platforms/BP_Platform.GroupTag` _array_element)))
      (`self.Interact` _array_element))))

(fn `UserConstructionScript`
  (`|ExecutionSequence`
    (:`then_0`
      (if (`self.StartsUp?`)
        (`PrimitiveComponent.SetMaterial` (`self.Platform`) 0 "/Game/Materials/Platforms/M_Blue.M_Blue")))
    (:`then_1`
      (if (`self.isShadow`)
        (`PrimitiveComponent.SetMaterial` (`self.Platform`) 0 "/Game/Materials/Platforms/M_Red.M_Red")))))